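; Base flower cannon enemy Blueprint, animated with PaperZD, that stays destroyed once killed.
; Shortly after BeginPlay it asks the GameInstance whether its CannonID is already destroyed, using the Lvl1 check, and removes itself if so.
; Events jump the animation to Attack or Hit nodes.
; Death reuses Hit, reports the ID to the GameInstance, then enables physics and launches the capsule upward.
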(event `self.ReceiveBeginPlay`
  (`KismetSystemLibrary.Delay` 0.2)
  (bind _destroy (message `/Game/SaveGame/BI_SG_Interface.Check it has to destroy (Enemy Lvl1)` (`GameplayStatics.GetGameInstance`) (`self.Cannon ID`)))
  (if _destroy
    (`self.K2_DestroyActor`)))

(event `self.PlayAttackAnim`
  (`PaperZDAnimInstance.JumpToNode` (`PaperZDAnimationComponent.AnimInstance` (`self.PaperZDAnimation`)) "Attack" "None"))

(event `self.PlayHitAnim`
  (`PaperZDAnimInstance.JumpToNode` (`PaperZDAnimationComponent.AnimInstance` (`self.PaperZDAnimation`)) "Hit" "None"))

(event `self.PlayDeadAnim`
  (bind _rootcapsule (`self.RootCapsule`))
  (`KismetSystemLibrary.PrintString` "Dead")
  (`PaperZDAnimInstance.JumpToNode` (`PaperZDAnimationComponent.AnimInstance` (`self.PaperZDAnimation`)) "Hit" "None")
  (`self.Inserting Actor Id`)
  (`PrimitiveComponent.SetCollisionEnabled` _rootcapsule "QueryAndPhysics")
  (`PrimitiveComponent.SetSimulatePhysics` _rootcapsule true)
  (`PrimitiveComponent.AddImpulse` (`self.RootCapsule`) (0.0 0.0 5000.0) "None" false))

(event `Inserting Actor Id`
  (message `/Game/SaveGame/BI_SG_Interface.Destroyed EnemyActor` (`GameplayStatics.GetGameInstance`) (`self.Cannon ID`)))

(fn `UserConstructionScript`)