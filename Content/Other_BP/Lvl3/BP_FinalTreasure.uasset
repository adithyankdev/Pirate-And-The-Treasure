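; BP_FinalTreasure is the Level 3 treasure actor that shows the finish screen when the player reaches it with the key.
; Its Box overlap checks the other actor against the BP_Player found in the world, then reads the GetKey flag from the GameInstance's game data.
; If the flag is set, it clears all widgets, adds WB_FinshWidget to the viewport and prints a debug string.
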(event `self.Box.OnComponentBeginOverlap`
  (params (OverlappedComponent :type "PrimitiveComponent Object Reference") (OtherActor :type "Actor Object Reference") (OtherComp :type "PrimitiveComponent Object Reference") (OtherBodyIndex :type Integer) (bFromSweep :type Boolean) (SweepResult :type "HitResult Structure (by ref)"))
  (bind _returnvalue (`GameplayStatics.GetActorOfClass` "/Game/Player/BP_Player.BP_Player_C"))
  (if (== _returnvalue OtherActor)
    (bind _sg_data (message `/Game/SaveGame/BI_SG_Interface.GetGameData` (`GameplayStatics.GetGameInstance`)))
    (if (`/Game/SaveGame/SG_PirateSaveGame.GetKey` _sg_data)
      (`WidgetLayoutLibrary.RemoveAllWidgets`)
      (bind _returnvalue_2 (`|CreateWidget` "/Game/Widgets/FinishGame/WB_FinshWidget.WB_FinshWidget_C"))
      (`UserWidget.AddToViewport` _returnvalue_2 0)
      (`KismetSystemLibrary.PrintString` "Hello"))))

(fn `UserConstructionScript`)