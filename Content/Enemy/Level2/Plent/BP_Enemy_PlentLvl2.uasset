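; BP_Enemy_PlentLvl2 is a level 2 plant enemy with PaperZD animations and persistent death state.
; Shortly after BeginPlay it asks the Game Instance whether its ActorID was already destroyed and, if so, removes itself; GetDestroyed reports that ID back.
; Hit and attack events jump animation nodes, and a hit also turns on capsule physics and launches the body with an impulse.
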(event `self.ReceiveBeginPlay`
  (`KismetSystemLibrary.Delay` 0.2)
  (bind _destroy (message `/Game/SaveGame/BI_SG_Interface.Check it has to destroy (Enemy Lvl1)` (`GameplayStatics.GetGameInstance`) (`self.Actor ID `)))
  (if _destroy
    (`self.K2_DestroyActor`)))

(event `self.GetDestroyed`
  (`self.Inserting Actor Id`))

(event `self.PlayHitAnim`
  (bind _capsulecomponent (`self.CapsuleComponent`))
  (`PaperZDAnimInstance.JumpToNode` (`PaperZDAnimationComponent.AnimInstance` (`self.PaperZDAnimation`)) "Hit" "None")
  (`PrimitiveComponent.SetCollisionEnabled` _capsulecomponent "QueryAndPhysics")
  (`PrimitiveComponent.SetSimulatePhysics` _capsulecomponent true)
  (`PrimitiveComponent.AddImpulse` _capsulecomponent (0.0 6000.0 6000.0) "None" false))

(event `self.PlayAttackAnim`
  (`PaperZDAnimInstance.JumpToNode` (`PaperZDAnimationComponent.AnimInstance` (`self.PaperZDAnimation`)) "Atk" "None"))

(event `Inserting Actor Id`
  (message `/Game/SaveGame/BI_SG_Interface.Destroyed EnemyActor` (`GameplayStatics.GetGameInstance`) (`self.Actor ID `)))

(fn `UserConstructionScript`)