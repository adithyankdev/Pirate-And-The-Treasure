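; Level 2 mushroom zombie enemy that plays PaperZD animations and stays removed once recorded as destroyed.
; Attack and hit events jump to nodes in its animation instance.
; GetDestroyed reports its ActorID to the game instance.
; After a short BeginPlay delay, it destroys itself if a save exists and the game instance flags that ID, using a check named for level 1 enemies.
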(event `self.ReceiveBeginPlay`
  (`KismetSystemLibrary.Delay` 0.2)
  (bind _slotname (message `/Game/SaveGame/BI_SG_Interface.GetSlotName` (`GameplayStatics.GetGameInstance`)))
  (bind _returnvalue (`GameplayStatics.DoesSaveGameExist` _slotname))
  (if _returnvalue
    (bind _destroy (message `/Game/SaveGame/BI_SG_Interface.Check it has to destroy (Enemy Lvl1)` (`GameplayStatics.GetGameInstance`) (`self.ActorID`)))
    (if _destroy
      (`self.K2_DestroyActor`))))

(event `self.PlayAttackAnim`
  (`PaperZDAnimInstance.JumpToNode` (`PaperZDAnimationComponent.AnimInstance` (`self.PaperZDAnimation`)) "Atk" "None"))

(event `self.PlayHitAnim`
  (`PaperZDAnimInstance.JumpToNode` (`PaperZDAnimationComponent.AnimInstance` (`self.PaperZDAnimation`)) "Hit" "None"))

(event `self.GetDestroyed`
  (`self.Inserting Actor ID `))

(event `Inserting Actor ID`
  (message `/Game/SaveGame/BI_SG_Interface.Destroyed EnemyActor` (`GameplayStatics.GetGameInstance`) (`self.ActorID`)))

(fn `UserConstructionScript`)