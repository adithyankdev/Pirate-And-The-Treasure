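; BP_Pig_Lvl1 is a level 1 pig enemy with PaperZD-style attack and hit animation jumps and persistence of its destroyed state.
; One second after BeginPlay, if a save exists, it asks the GameInstance whether its ActorID should be destroyed.
; Only on that destroy branch does it also read the saved difficulty, after calling DestroyActor.
; GetDestroyed reports the ActorID to the GameInstance.
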(event `self.PlayAttackAnim`
  (`PaperZDAnimInstance.JumpToNode` (`PaperZDAnimationComponent.AnimInstance` (`self.Pig Animation`)) "Attack" "None"))

(event `self.PlayHitAnim`
  (`PaperZDAnimInstance.JumpToNode` (`PaperZDAnimationComponent.AnimInstance` (`self.Pig Animation`)) "Hit" "None"))

(event `self.ReceiveBeginPlay`
  (`KismetSystemLibrary.Delay` 1.0)
  (bind _slotname (message `/Game/SaveGame/BI_SG_Interface.GetSlotName` (`GameplayStatics.GetGameInstance`)))
  (bind _returnvalue (`GameplayStatics.DoesSaveGameExist` _slotname))
  (if _returnvalue
    (bind _destroy (message `/Game/SaveGame/BI_SG_Interface.Check it has to destroy (Enemy Lvl1)` (`GameplayStatics.GetGameInstance`) (`self.Actor ID`)))
    (if _destroy
      (`self.K2_DestroyActor`)
      (bind _sg_data (message `/Game/SaveGame/BI_SG_Interface.GetGameData` (`GameplayStatics.GetGameInstance`)))
      (set `self.DIFFICULTY` (`/Game/SaveGame/SG_PirateSaveGame.GameDifficulty` _sg_data)))))

(event `Inserting Actor ID`
  (message `/Game/SaveGame/BI_SG_Interface.Destroyed EnemyActor` (`GameplayStatics.GetGameInstance`) (`self.Actor ID`)))

(event `self.GetDestroyed`
  (`self.Inserting Actor ID`))

(fn `UserConstructionScript`)