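; BP_PinkStar_Lvl1 is the Blueprint for the Level 1 Pink Star enemy, handling its animation triggers and persistent destruction.
; Attack and hit events jump its animation instance directly to the matching state nodes.
; Shortly after BeginPlay it asks the GameInstance whether its ActorID was already destroyed and removes itself if so.
; GetDestroyed reports that ActorID to the GameInstance so the defeat is remembered.
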(event `self.PlayAttackAnim`
  (`PaperZDAnimInstance.JumpToNode` (`PaperZDAnimationComponent.AnimInstance` (`self.PinkStar Animation`)) "Attack" "None"))

(event `self.PlayHitAnim`
  (`PaperZDAnimInstance.JumpToNode` (`PaperZDAnimationComponent.AnimInstance` (`self.PinkStar Animation`)) "Hit" "None"))

(event `self.ReceiveBeginPlay`
  (`KismetSystemLibrary.Delay` 0.2)
  (bind _destroy (message `/Game/SaveGame/BI_SG_Interface.Check it has to destroy (Enemy Lvl1)` (`GameplayStatics.GetGameInstance`) (`self.Actor ID`)))
  (if _destroy
    (`self.K2_DestroyActor`)))

(event `self.GetDestroyed`
  (`self.Inserting Actor Id`))

(event `Inserting Actor Id`
  (message `/Game/SaveGame/BI_SG_Interface.Destroyed EnemyActor` (`GameplayStatics.GetGameInstance`) (`self.Actor ID`)))

(fn `UserConstructionScript`)