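; BP_CollectableMap is a map collectable with a Paper2D flipbook, whose collected state is tracked by ActorID in the Game Instance.
; Shortly after BeginPlay it asks the Game Instance whether that ID was already collected, and destroys itself if so.
; CollectMapAnimation switches to the collected flipbook, while GetDestroyed only registers the ID with the Game Instance.
; Overlap detection and the calls to these events are not handled here.
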(event `self.CollectMapAnimation`
  (`PaperFlipbookComponent.SetFlipbook` (`self.PaperFlipbook`) "/Game/Collectable/MiniMap/Flipbooks/FB_Map_Collected.FB_Map_Collected"))

(event `self.ReceiveBeginPlay`
  (`KismetSystemLibrary.Delay` 0.2)
  (bind _destroy (message `/Game/SaveGame/BI_SG_Interface.Check if it need Destroy(Collectables)` (`GameplayStatics.GetGameInstance`) (`self.ActorID`)))
  (if _destroy
    (`self.K2_DestroyActor`)))

(event `self.GetDestroyed`
  (`self.InsertingActorID`))

(event `InsertingActorID`
  (message `/Game/SaveGame/BI_SG_Interface.DestroyedCollectables` (`GameplayStatics.GetGameInstance`) (`self.ActorID`)))

(fn `UserConstructionScript`)