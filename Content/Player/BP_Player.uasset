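; Player Blueprint that restores a saved position, plays combat animations and switches UI screens.
; On BeginPlay, if a save exists, it applies the transform from the game instance's save data.
; Attack events alternate two animations via FlipFlop and JumpToNode on the anim instance, which also handles hit reactions.
; Shop and end-game events swap the in-game HUD for their widgets, while the speed boost event is empty.
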(event `self.ShopWidgetTrigger`
  (bind _foundwidgets (`WidgetBlueprintLibrary.GetAllWidgetsOfClass` "/Game/Widgets/OnGame/WB_OnGame.WB_OnGame_C"))
  (`Widget.RemoveFromParent` _foundwidgets)
  (bind _returnvalue (`|CreateWidget` "/Game/Widgets/Shop/WB_OnShop.WB_OnShop_C"))
  (`UserWidget.AddToViewport` _returnvalue 0))

(event `self.ReceiveBeginPlay`
  (bind _returnvalue (`GameplayStatics.DoesSaveGameExist` "Save1"))
  (if _returnvalue
    (bind _sg_data (message `/Game/SaveGame/BI_SG_Interface.GetGameData` (`GameplayStatics.GetGameInstance`)))
    (bind _savegame_data_playerlocation (break `/Game/SaveGame/Struct_SaveInfo` (`/Game/SaveGame/SG_PirateSaveGame.SaveGame Data` _sg_data)))
    (`self.SetPlayerInfo` _savegame_data_playerlocation)))

(event `self.ReceiveTick`
  (params (DeltaSeconds :type "Float (single-precision)")))

(event `self.PlayAttackAnim`
  (bind _animinstance (`PaperZDAnimationComponent.AnimInstance` (`self.PlayerAnimation`)))
  (`/Engine/EditorBlueprintResources/StandardMacros.FlipFlop`
    (:`A`
      (`PaperZDAnimInstance.JumpToNode` _animinstance "Attack1" "None"))
    (:`B`
      (`PaperZDAnimInstance.JumpToNode` _animinstance "Attack2" "None"))))

(event `self.PlayHitAnim`
  (`PaperZDAnimInstance.JumpToNode` (`PaperZDAnimationComponent.AnimInstance` (`self.PlayerAnimation`)) "Hit" "None"))

(event `self.CallEndWidget`
  (bind _foundwidgets (`WidgetBlueprintLibrary.GetAllWidgetsOfClass` "/Game/Widgets/OnGame/WB_OnGame.WB_OnGame_C"))
  (`Widget.RemoveFromParent` _foundwidgets)
  (bind _returnvalue (`|CreateWidget` "/Game/Widgets/EndGame/WB_EndGame.WB_EndGame_C"))
  (`UserWidget.AddToViewport` _returnvalue 0))

(event `self.ActivateSpeedBoost`)

(fn `SetPlayerInfo`
  (params (Transform :type "Transform Structure"))
  (`self.K2_SetActorTransform` Transform))

(fn `UserConstructionScript`)