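; Flag checkpoint actor that records the player's progress in the Game Instance when BP_Player enters its box trigger.
; On overlap, it gathers the player's transform, speed potion and projectile counts, plus coins from the Game Instance's game data and the current level name.
; It passes that snapshot to the Game Instance through SetPlayerInfoMessage.
; The invalid-player branch loops back to the cast.
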(event `self.Box.OnComponentBeginOverlap`
  (params (OverlappedComponent :type "PrimitiveComponent Object Reference") (OtherActor :type "Actor Object Reference") (OtherComp :type "PrimitiveComponent Object Reference") (OtherBodyIndex :type Integer) (bFromSweep :type Boolean) (SweepResult :type "HitResult Structure (by ref)"))
  (bind _returnvalue (`GameplayStatics.GetGameInstance`))
  (bind _as_bp_player (`self.As BP Player`))
  (bind _asbp_player (cast `/Game/Player/BP_Player` OtherActor :!label _label))
  (`/Engine/EditorBlueprintResources/StandardMacros.IsValid` _asbp_player
    (:`Is Valid`
      (set `self.As BP Player` _asbp_player)
      (bind _sg_data (message `/Game/SaveGame/BI_SG_Interface.GetGameData` _returnvalue))
      (bind _returnvalue_2 (`GameplayStatics.GetCurrentLevelName` true))
      (message `/Game/SaveGame/BI_SG_Interface.SetPlayerInfo` _returnvalue (make `/Game/SaveGame/Struct_SaveInfo` (`self.GetTransform` _as_bp_player) (`/Game/SaveGame/SG_PirateSaveGame.Coins` _sg_data) (`PlayerPirate.SpeedBoostCount` _as_bp_player) 0 (`PlayerPirate.ProjectileCount` _as_bp_player)) _returnvalue_2))
    (:`Is Not Valid`
      (goto _label))))

(fn `UserConstructionScript`)